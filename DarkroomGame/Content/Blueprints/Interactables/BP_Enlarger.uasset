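; Interactable darkroom enlarger that exposes photos placed on it and fails those left too long.
; Interaction snaps an eligible BPI_Photo item onto it or toggles the light.
; When lit and GI_Main allows developing, a timer advances the photo's state while Tick fills a widget progress bar, then counts toward overexposure failure.
; ClearValues resets the enlarger and fails any photo still mid-exposure.
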(event `self.ReceiveBeginPlay`
  (bind _aswbp_progress_bar (cast `/Game/UI/WBP_ProgressBar` (`WidgetComponent.GetUserWidgetObject` (`self.ProgressBar`))))
  (set `self.ProgressBarActor` _aswbp_progress_bar))

(event `CallExposePhoto`
  (`self.ExposePhoto` (`self.PhotoActor`)))

(event `/Game/Blueprints/Items/BPI_Interactable.HandleInteraction`
  (params (HeldItemREF :type "Actor Object Reference"))
  (if (and (not (`KismetSystemLibrary.IsValid` (`self.PhotoActor`))) (`KismetSystemLibrary.DoesImplementInterface` HeldItemREF "/Game/Blueprints/Photos/BPI_Photo.BPI_Photo_C"))
    (bind _photostate (message `/Game/Blueprints/Photos/BPI_Photo.GetPhotoState` HeldItemREF))
    (if (`|EnumEquality` _photostate "NewEnumerator0")
      (`self.PlacePhoto` HeldItemREF)
      (if (`self.bIsOn`) :!label _label
        (bind _asgi_main (cast `/Game/Blueprints/Gameplay/GI_Main` (`GameplayStatics.GetGameInstance`)))
        (if (`/Game/Blueprints/Gameplay/GI_Main.bCanDevelopPhoto` _asgi_main)
          (bind _returnvalue (`KismetSystemLibrary.K2_SetTimerDelegate` (delegate `CallExposePhoto`) (`self.ExposureTimer`)))
          (set `self.Is Developing Photo` true))))
    (else
      (`self.ToggleEnlarger`)
      (`/Engine/EditorBlueprintResources/StandardMacros.IsValid` (`self.PhotoActor`)
        (:`Is Valid`
          (goto _label))))))

(event `/Game/Blueprints/Items/BPI_Interactable.ClearValues`
  (if (`self.Is Developing Photo`)
    (`self.SetPhotoFailed`))
  (`self.ClearValuesFunction`)
  (`KismetSystemLibrary.K2_ClearAndInvalidateTimerHandle` (stale `/Game/Blueprints/Items/BPI_Interactable.HandleInteraction` _returnvalue)))

(event `self.ReceiveTick`
  (params (DeltaSeconds :type "Float (single-precision)"))
  (if (`self.Is Developing Photo`)
    (set `self.ProgressValue` (`KismetMathLibrary.FClamp` (+ (`self.ProgressValue`) (/ DeltaSeconds (`self.ExposureTimer`)))))
    (`self.UpdateProgressBar`)
    (elif (>= (`self.ProgressValue`) 1.0)
      (bind _output_get (set `self.OverexposureElapsed` (+ (`self.OverexposureElapsed`) DeltaSeconds)))
      (if (>= _output_get (`self.OverexposureTimer`))
        (`/Engine/EditorBlueprintResources/StandardMacros.DoOnce` false
          (:`Completed`
            (`self.SetPhotoFailed`)))))))

(fn `ClearValuesFunction`
  (bind _progressbar (`/Game/UI/WBP_ProgressBar.ProgressBar` (`self.ProgressBarActor`)))
  (set `self.bHasPhoto` false)
  (set `self.bIsPhotoExposed` false)
  (set `self.PhotoActor` null)
  (`PrimitiveComponent.SetCollisionEnabled` (`self.ItemMesh`) "QueryAndPhysics")
  (`ProgressBar.SetPercent` _progressbar 0.0)
  (`ProgressBar.SetFillColorAndOpacity` _progressbar (struct :`R` 0.054902 :`G` 0.564706 :`B` 0.176471 :`A` 1.0))
  (set `self.OverexposureElapsed` 0.0)
  (set `self.ProgressValue` 0.0))

(fn `ExposePhoto`
  (params (PhotoToExpose :type "Actor Object Reference"))
  (message `/Game/Blueprints/Photos/BPI_Photo.ChangePhotoState` PhotoToExpose "NewEnumerator1")
  (set `self.bIsPhotoExposed` true)
  (`KismetSystemLibrary.PrintString` "Photo Exposed!")
  (`PrimitiveComponent.SetCollisionEnabled` (`self.ItemMesh`) "NoCollision")
  (set `self.Is Developing Photo` false))

(fn `PlacePhoto`
  (params (PhotoREF :type "Actor Object Reference"))
  (bind _photopoint (`self.PhotoPoint`))
  (`self.K2_SetActorLocationAndRotation` PhotoREF (`SceneComponent.K2_GetComponentLocation` _photopoint) (`SceneComponent.K2_GetComponentRotation` _photopoint) false false)
  (bind _output_get (set `self.PhotoActor` PhotoREF))
  (message `/Game/Blueprints/Photos/BPI_Photo.ConnectEnlarger` _output_get self)
  (`PrimitiveComponent.SetCollisionEnabled` (`self.ItemMesh`) "NoCollision"))

(fn `SetPhotoFailed`
  (bind _photoactor (`self.PhotoActor`))
  (`/Engine/EditorBlueprintResources/StandardMacros.IsValid` _photoactor
    (:`Is Valid`
      (message `/Game/Blueprints/Photos/BPI_Photo.ChangePhotoState` _photoactor "NewEnumerator4")
      (`ProgressBar.SetFillColorAndOpacity` (`/Game/UI/WBP_ProgressBar.ProgressBar` (`self.ProgressBarActor`)) (struct :`R` 0.854167 :`G` 0.025928 :`B` 0.059924 :`A` 1.0))
      (set `self.bIsOverexposing` false)
      (`GameplayStatics.PlaySound2D` "/Engine/VREditor/Sounds/UI/Invalid_Action.Invalid_Action" 1.0 1.0 0.0 null null)
      (`KismetSystemLibrary.PrintString` "Photo Failed!")
      (set `self.Is Developing Photo` false))))

(fn `ToggleEnlarger`
  (bind _output_get (set `self.bIsOn` (not (`self.bIsOn`))))
  (`SceneComponent.SetVisibility` (`self.SpotLight`) _output_get false)
  (`PrimitiveComponent.SetMaterial` (`self.On/Off Light`) 0 (select `bool` (`self.bIsOn`) :`false` "/Engine/VREditor/BasicMeshes/MI_Cube_03.MI_Cube_03" :`true` "/Engine/EngineDebugMaterials/VertexColorViewMode_GreenOnly.VertexColorViewMode_GreenOnly" :!type "MaterialInterface Object Reference"))
  (`GameplayStatics.PlaySound2D` "/Engine/VREditor/Sounds/UI/Click_on_Button.Click_on_Button" 1.0 1.0 0.0 null null))

(fn `UpdateProgressBar`
  (`ProgressBar.SetPercent` (`/Game/UI/WBP_ProgressBar.ProgressBar` (`self.ProgressBarActor`)) (`self.ProgressValue`)))

(fn `UserConstructionScript`
  (`parent.UserConstructionScript`))