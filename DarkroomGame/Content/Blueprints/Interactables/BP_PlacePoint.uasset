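; BP_PlacePoint is an interactable snap point that accepts a single item type, such as Chemical, Vessel or Clip.
; PlaceItem queries the incoming item's type, and on a match moves it to the point's location and rotation, then sets IsPlaced on its BP_ItemBase.
; Helper functions expose the accepted type and map it to the corresponding item Blueprint class.
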(event `/Game/Blueprints/Interactables/BPI_PlacePoint.PlaceItem`
  (params (ItemToPlace :type "Actor Object Reference"))
  (bind _itemtype (message `/Game/Blueprints/Items/BPI_Interactable.GetItemType` ItemToPlace))
  (bind _bcanacceptitem (`self.CanAcceptItem` _itemtype))
  (if _bcanacceptitem
    (`self.K2_SetActorLocationAndRotation` ItemToPlace (`self.K2_GetActorLocation`) (`self.K2_GetActorRotation`) false false)
    (bind _asbp_item_base (cast `/Game/Blueprints/Items/BP_ItemBase` ItemToPlace))
    (set `/Game/Blueprints/Items/BP_ItemBase.bIsPlaced` true _asbp_item_base)))

(fn `CanAcceptItem`
  (params (ItemType :type "/Game/Blueprints/Items/EItemType Enum" :default "NewEnumerator4"))
  (returns (bCanAcceptItem :type Boolean))
  (return (`|EnumEquality` ItemType (`self.AcceptedType`))))

(fn `GetAcceptedItemType`
  (returns (ItemType :type "/Game/Blueprints/Items/EItemType Enum"))
  (return (`self.AcceptedType`)))

(fn `SetItemClass`
  (switch `/Game/Blueprints/Items/EItemType` (`self.AcceptedType`)
    (:`NewEnumerator0`
      (set `self.ItemClass` "/Game/Blueprints/Items/BP_Chemical.BP_Chemical_C"))
    (:`NewEnumerator1`
      (set `self.ItemClass` "/Game/Blueprints/Items/BP_Vessel.BP_Vessel_C"))
    (:`NewEnumerator2`
      (set `self.ItemClass` "/Game/Blueprints/Items/BP_Clip.BP_Clip_C"))))

(fn `UserConstructionScript`)