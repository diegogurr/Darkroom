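; Inventory component that stores items in an array and tracks a selected slot for scrolling.
; Helper functions add, remove, look up and fetch items, and report when the array length equals the maximum size.
; AddItem prints a warning once the length exceeds that maximum, so it accepts one item beyond it.
; ScrollInventory steps the index by direction sign, clamped to maximum capacity rather than item count, and returns that item.
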(fn `AddItem`
  (params (NewItem :type "/Game/Blueprints/Items/FItemData Structure"))
  (if (<= (`KismetArrayLibrary.Array_Length` (`self.Inventory`)) (`self.MaxInventorySize`))
    (`KismetArrayLibrary.Array_Add` (`self.Inventory`) NewItem)
    (else
      (`KismetSystemLibrary.PrintString` "Inventory is full!"))))

(fn `GetItemAtIndex`
  (params (SelectedItemIndex :type Integer))
  (returns (SelectedItemData :type "/Game/Blueprints/Items/FItemData Structure"))
  (return (`|GetArrayItem` (`self.Inventory`) SelectedItemIndex)))

(fn `HasItem`
  (params (ItemToCheck :type "/Game/Blueprints/Items/FItemData Structure"))
  (returns (ReturnValue :type Boolean))
  (return (`KismetArrayLibrary.Array_Contains` (`self.Inventory`) ItemToCheck)))

(fn `IsInventoryFull`
  (returns (bIsInventoryFull :type Boolean))
  (return (== (`KismetArrayLibrary.Array_Length` (`self.Inventory`)) (`self.MaxInventorySize`))))

(fn `RemoveItem`
  (params (ItemToRemove :type "/Game/Blueprints/Items/FItemData Structure"))
  (`KismetArrayLibrary.Array_RemoveItem` (`self.Inventory`) ItemToRemove))

(fn `ScrollInventory`
  (params (Direction :type "Float (double-precision)"))
  (returns (SelectedItemData :type "/Game/Blueprints/Items/FItemData Structure"))
  (bind _selected_inventory_item_index (`self.Selected Inventory Item Index`))
  (bind _returnvalue (- (`self.MaxInventorySize`) 1))
  (if (not (== (`KismetArrayLibrary.Array_Length` (`self.Inventory`)) 0))
    (`/Engine/EditorBlueprintResources/StandardMacros.CompareFloat` Direction
      (:`>`
        (bind _result (`/Engine/EditorBlueprintResources/StandardMacros.IncrementInt` _selected_inventory_item_index)
          (:`  `
            (bind _output_get (set `self.Selected Inventory Item Index` (`KismetMathLibrary.Clamp` _result 0 _returnvalue)))
            (bind _selecteditemdata (`self.GetItemAtIndex` _output_get))
            (return _selecteditemdata))))
      (:`<`
        (bind _result_2 (`/Engine/EditorBlueprintResources/StandardMacros.DecrementInt` _selected_inventory_item_index)
          (:`  `
            (bind _output_get_2 (set `self.Selected Inventory Item Index` (`KismetMathLibrary.Clamp` _result_2 0 _returnvalue)))
            (bind _selecteditemdata_2 (`self.GetItemAtIndex` _output_get_2))
            (return _selecteditemdata_2)))))))