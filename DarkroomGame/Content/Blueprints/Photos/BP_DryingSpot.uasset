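; Clothesline drying spot where the player hangs a photo to dry in the photo development process.
; An interaction first snaps a pin item to the pin point, then accepts one photo in the required phase at the photo point.
; The placed photo receives a reference to the spot, and a timer changes its state once drying ends.
; ClearValues releases the photo reference and cancels the timer, leaving the pin in place.
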(event `/Game/Blueprints/Items/BPI_Interactable.HandleInteraction`
  (params (HeldItemREF :type "Actor Object Reference"))
  (if (`self.bHasClothesPin`)
    (`/Engine/EditorBlueprintResources/StandardMacros.IsValid` (`self.PhotoActor`)
      (:`Is Not Valid`
        (if (`KismetSystemLibrary.DoesImplementInterface` HeldItemREF "/Game/Blueprints/Photos/BPI_Photo.BPI_Photo_C")
          (bind _photophase (message `/Game/Blueprints/Photos/BPI_Photo.GetPhotoPhase` HeldItemREF))
          (if (`|EnumEquality` _photophase "NewEnumerator4")
            (`self.PlacePhoto` HeldItemREF)
            (bind _returnvalue (`KismetSystemLibrary.K2_SetTimerDelegate` (delegate `CallExposePhoto`) (`self.DryingTimer`)))))))
    (else
      (bind _itemtype (message `/Game/Blueprints/Items/BPI_Interactable.GetItemType` HeldItemREF))
      (if (`|EnumEquality` _itemtype "NewEnumerator2")
        (`self.PlacePin` HeldItemREF)))))

(event `/Game/Blueprints/Items/BPI_Interactable.ClearValues`
  (`self.ClearValuesFunction`)
  (`KismetSystemLibrary.K2_ClearAndInvalidateTimerHandle` (stale `/Game/Blueprints/Items/BPI_Interactable.HandleInteraction` _returnvalue)))

(event `CallExposePhoto`
  (`self.DryPhoto` (`self.PhotoActor`)))

(fn `CanAcceptItem`
  (params (ItemType :type "/Game/Blueprints/Items/EItemType Enum" :default "NewEnumerator4"))
  (returns (bCanAcceptItem :type Boolean))
  (return false))

(fn `CanInteract`
  (returns (CanInteract :type Boolean))
  (return false))

(fn `CanPickup`
  (returns (bCanPickup :type Boolean))
  (return false))

(fn `ClearValuesFunction`
  (set `self.PhotoActor` null))

(fn `DryPhoto`
  (params (PhotoToExpose :type "Actor Object Reference"))
  (message `/Game/Blueprints/Photos/BPI_Photo.ChangePhotoState` PhotoToExpose "NewEnumerator3")
  (`KismetSystemLibrary.PrintString` "Photo developed!"))

(fn `GetAcceptedItemType`
  (returns (ItemType :type "/Game/Blueprints/Items/EItemType Enum"))
  (return "NewEnumerator4"))

(fn `GetItemData`
  (returns (ItemData :type "/Game/Blueprints/Items/FItemData Structure"))
  (return (make `/Game/Blueprints/Items/FItemData` "Clothesline")))

(fn `GetItemType`
  (returns (ItemType :type "/Game/Blueprints/Items/EItemType Enum"))
  (return "NewEnumerator4"))

(fn `PlacePhoto`
  (params (PhotoREF :type "Actor Object Reference"))
  (bind _photopoint (`self.PhotoPoint`))
  (`self.K2_SetActorLocationAndRotation` PhotoREF (`SceneComponent.K2_GetComponentLocation` _photopoint) (`SceneComponent.K2_GetComponentRotation` _photopoint) false false)
  (bind _output_get (set `self.PhotoActor` PhotoREF))
  (message `/Game/Blueprints/Photos/BPI_Photo.ConnectClothesline` _output_get self))

(fn `PlacePin`
  (params (PinREF :type "Actor Object Reference"))
  (bind _pinpoint (`self.PinPoint`))
  (`self.K2_SetActorLocationAndRotation` PinREF (`SceneComponent.K2_GetComponentLocation` _pinpoint) (`SceneComponent.K2_GetComponentRotation` _pinpoint) false false)
  (set `self.bHasClothesPin` true)
  (bind _asbp_clip (cast `/Game/Blueprints/Items/BP_Clip` PinREF))
  (set `/Game/Blueprints/Items/BP_ItemBase.bIsPlaced` true _asbp_clip))

(fn `UserConstructionScript`)