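; BP_Photo is a pickup item representing a photo that moves through darkroom processing with an enlarger and chemical vessels.
; It stores a photo state and phase through setter events and getters, and supplies its item data and allows pickup only when not placed.
; On interaction it clears the value messages on any connected vessel, and on the enlarger in one specific state, then drops those references.
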(event `/Game/Blueprints/Photos/BPI_Photo.ChangePhotoState`
  (params (NewPhotoState :type "/Game/Blueprints/Photos/EPhotoState Enum" :default "NewEnumerator0"))
  (set `self.CurrentState` NewPhotoState))

(event `/Game/Blueprints/Photos/BPI_Photo.ChangePhotoPhase`
  (params (NewPhotoPhase :type "/Game/Blueprints/Photos/EPhotoPhase Enum" :default "NewEnumerator0"))
  (set `self.CurrentPhotoPhase` NewPhotoPhase))

(event `/Game/Blueprints/Photos/BPI_Photo.ConnectEnlarger`
  (params (EnlargerREF :type "Actor Object Reference"))
  (set `self.ConnectedEnlarger` EnlargerREF))

(event `/Game/Blueprints/Photos/BPI_Photo.ConnectVessel`
  (params (VesselREF :type "Actor Object Reference"))
  (set `self.ConnectedVessel` VesselREF))

(event `/Game/Blueprints/Items/BPI_Interactable.HandleInteraction`
  (params (HeldItemREF :type "Actor Object Reference"))
  (bind _connectedenlarger (`self.ConnectedEnlarger`))
  (bind _connectedvessel (`self.ConnectedVessel`))
  (`|ExecutionSequence`
    (:`then_0`
      (if (`|EnumEquality` (`self.CurrentState`) "NewEnumerator1")
        (`/Engine/EditorBlueprintResources/StandardMacros.IsValid` _connectedenlarger
          (:`Is Valid`
            (message `/Game/Blueprints/Items/BPI_Interactable.ClearValues` _connectedenlarger)
            (set `self.ConnectedEnlarger` null)))))
    (:`then_1`
      (`/Engine/EditorBlueprintResources/StandardMacros.IsValid` _connectedvessel
        (:`Is Valid`
          (message `/Game/Blueprints/Items/BPI_Interactable.ClearValues` _connectedvessel)
          (set `self.ConnectedVessel` null))))))

(fn `CanPickup`
  (returns (bCanPickup :type Boolean))
  (return (not (`self.bIsPlaced`))))

(fn `GetItemData`
  (returns (ItemData :type "/Game/Blueprints/Items/FItemData Structure"))
  (return (make `/Game/Blueprints/Items/FItemData` "Photo")))

(fn `GetPhotoPhase`
  (returns (PhotoPhase :type "/Game/Blueprints/Photos/EPhotoPhase Enum"))
  (return (`self.CurrentPhotoPhase`)))

(fn `GetPhotoState`
  (returns (PhotoState :type "/Game/Blueprints/Photos/EPhotoState Enum"))
  (return (`self.CurrentState`)))

(fn `UserConstructionScript`
  (`parent.UserConstructionScript`))