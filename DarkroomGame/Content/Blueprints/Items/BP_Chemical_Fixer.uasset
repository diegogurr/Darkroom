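; BP_Chemical_Fixer is an item Blueprint for a fixer chemical that holds a liquid type and an empty state.
; It exposes getters for the chemical type and empty state, alongside a SetIsEmpty event that stores the new state.
; When set empty, the event swaps the item mesh's first material to Black, with no branch restoring it when refilled.
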(event `/Game/Blueprints/Items/BPI_Liquid.SetIsEmpty`
  (params (NewIsEmpty :type Boolean))
  (bind _output_get (set `self.bIsEmpty` NewIsEmpty))
  (if _output_get
    (`PrimitiveComponent.SetMaterial` (`self.ItemMesh`) 0 "/Game/Assets/Materials/Black.Black")))

(fn `GetIsEmpty`
  (returns (bIsEmpty :type Boolean))
  (return (`self.bIsEmpty`)))

(fn `GetLiquidType`
  (returns (LiquidType :type "/Game/Blueprints/Items/EChemicalType Enum"))
  (return (`self.ChemicalType`)))

(fn `UserConstructionScript`
  (`parent.UserConstructionScript`))