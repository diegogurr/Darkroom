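; BP_Vessel is a darkroom vessel item that, once placed, can be filled with a chemical to develop photos.
; Interaction fills it from liquid items or docks a photo whose phase matches the chemical (Developer, Stop Bath, Fixer, Water) through interface messages.
; A timer advances the photo phase while Tick drives a widget progress bar, then counts overexposure towards failure.
; ClearValues resets colliders and progress, cancels the timer and fails the photo.
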(event `self.ReceiveBeginPlay`
  (bind _aswbp_progress_bar (cast `/Game/UI/WBP_ProgressBar` (`WidgetComponent.GetUserWidgetObject` (`self.ProgressBar`))))
  (set `self.ProgressBarActor` _aswbp_progress_bar))

(event `/Game/Blueprints/Items/BPI_Interactable.HandleInteraction`
  (params (HeldItemREF :type "Actor Object Reference"))
  (if (`KismetSystemLibrary.DoesImplementInterface` HeldItemREF "/Game/Blueprints/Items/BPI_Liquid.BPI_Liquid_C")
    (bind _liquidtype (message `/Game/Blueprints/Items/BPI_Liquid.GetLiquidType` HeldItemREF))
    (bind _bfilledsuccessful (`self.FillVessel` _liquidtype))
    (if _bfilledsuccessful
      (`/Engine/EditorBlueprintResources/StandardMacros.IsValid` HeldItemREF
        (:`Is Valid`
          (`self.K2_DestroyActor` HeldItemREF))))
    (elif (`KismetSystemLibrary.DoesImplementInterface` HeldItemREF "/Game/Blueprints/Photos/BPI_Photo.BPI_Photo_C")
      (if (`self.bIsFilled`)
        (bind _photostate (message `/Game/Blueprints/Photos/BPI_Photo.GetPhotoState` HeldItemREF))
        (if (`|EnumEquality` _photostate "NewEnumerator1")
          (bind _photophase (message `/Game/Blueprints/Photos/BPI_Photo.GetPhotoPhase` HeldItemREF))
          (bind _photophase_2 (`self.GetAcceptedPhotoPhase`))
          (if (`|EnumEquality` _photophase _photophase_2)
            (`self.PlacePhoto` HeldItemREF)
            (bind _returnvalue (`KismetSystemLibrary.K2_SetTimerDelegate` (delegate `CallExposePhoto`) (`self.ImmersionTimer`)))
            (set `self.bIsDevelopingPhoto` true)))))))

(event `CallExposePhoto`
  (`self.DevelopPhoto` (`self.PhotoActor`)))

(event `/Game/Blueprints/Items/BPI_Interactable.ClearValues`
  (`self.ClearValuesFunction`)
  (`KismetSystemLibrary.K2_ClearAndInvalidateTimerHandle` (stale `/Game/Blueprints/Items/BPI_Interactable.HandleInteraction` _returnvalue))
  (`self.SetPhotoFailed`)
  (`KismetSystemLibrary.PrintString` "Took out early. Photo Failed!"))

(event `self.ReceiveTick`
  (params (DeltaSeconds :type "Float (single-precision)"))
  (if (`self.bIsDevelopingPhoto`)
    (set `self.ProgressValue` (`KismetMathLibrary.FClamp` (+ (`self.ProgressValue`) (/ DeltaSeconds (`self.ImmersionTimer`)))))
    (`self.UpdateProgressBar`)
    (elif (>= (`self.ProgressValue`) 1.0)
      (bind _output_get (set `self.OverexposureElapsed` (+ (`self.OverexposureElapsed`) DeltaSeconds)))
      (if (>= _output_get (`self.OverexposureTimer`))
        (`self.SetPhotoFailed`)))))

(fn `CanInteract`
  (returns (CanInteract :type Boolean))
  (return true))

(fn `CanPickup`
  (returns (bCanPickup :type Boolean))
  (return (not (`self.bIsPlaced`))))

(fn `ClearValuesFunction`
  (bind _progressbar (`/Game/UI/WBP_ProgressBar.ProgressBar` (`self.ProgressBarActor`)))
  (`PrimitiveComponent.SetCollisionEnabled` (`self.HitBox`) "QueryAndPhysics")
  (`PrimitiveComponent.SetCollisionEnabled` (`self.LiquidMesh`) "QueryAndPhysics")
  (`PrimitiveComponent.SetCollisionEnabled` (`self.ItemMesh`) "QueryAndPhysics")
  (`ProgressBar.SetPercent` _progressbar 0.0)
  (`ProgressBar.SetFillColorAndOpacity` _progressbar (struct :`R` 0.054902 :`G` 0.564706 :`B` 0.176471 :`A` 1.0))
  (set `self.OverexposureElapsed` 0.0)
  (set `self.ProgressValue` 0.0)
  (set `self.bIsDevelopingPhoto` false))

(fn `DeactivateColliders`
  (`PrimitiveComponent.SetCollisionEnabled` (`self.HitBox`) "NoCollision")
  (`PrimitiveComponent.SetCollisionEnabled` (`self.LiquidMesh`) "NoCollision")
  (`PrimitiveComponent.SetCollisionEnabled` (`self.ItemMesh`) "NoCollision"))

(fn `DevelopPhoto`
  (params (PhotoToExpose :type "Actor Object Reference"))
  (switch `/Game/Blueprints/Items/EChemicalType` (`self.ChemicalType`)
    (:`NewEnumerator0`
      (message `/Game/Blueprints/Photos/BPI_Photo.ChangePhotoPhase` PhotoToExpose "NewEnumerator1"))
    (:`NewEnumerator1`
      (message `/Game/Blueprints/Photos/BPI_Photo.ChangePhotoPhase` PhotoToExpose "NewEnumerator2"))
    (:`NewEnumerator2`
      (message `/Game/Blueprints/Photos/BPI_Photo.ChangePhotoPhase` PhotoToExpose "NewEnumerator3"))
    (:`NewEnumerator3`
      (message `/Game/Blueprints/Photos/BPI_Photo.ChangePhotoPhase` PhotoToExpose "NewEnumerator4")))
  (`self.DeactivateColliders`)
  (`KismetSystemLibrary.PrintString` "Photo changed phase!")
  (set `self.bIsDevelopingPhoto` false))

(fn `FillVessel`
  (params (NewChemicalType :type "/Game/Blueprints/Items/EChemicalType Enum" :default "NewEnumerator4"))
  (returns (bFilledSuccessful :type Boolean))
  (if (`self.bIsPlaced`)
    (set `self.ChemicalType` NewChemicalType)
    (`SceneComponent.SetVisibility` (`self.LiquidMesh`) true false)
    (`PrimitiveComponent.SetMaterial` (`self.LiquidMesh`) 0 (select `/Game/Blueprints/Items/EChemicalType` NewChemicalType :`NewEnumerator0` "/Game/Assets/Materials/M_Transparent.M_Transparent" :`NewEnumerator1` "/Game/Assets/Materials/M_Transparent_Gold.M_Transparent_Gold" :`NewEnumerator2` "/Game/Assets/Materials/M_Transparent_Black.M_Transparent_Black" :`NewEnumerator3` "/Game/Assets/Materials/M_Transparent_Blue.M_Transparent_Blue" :!type "MaterialInterface Object Reference"))
    (set `self.bIsFilled` true)
    (return true)))

(fn `GetAcceptedPhotoPhase`
  (returns (PhotoPhase :type "/Game/Blueprints/Photos/EPhotoPhase Enum"))
  (switch `/Game/Blueprints/Items/EChemicalType` (`self.ChemicalType`)
    (:`NewEnumerator0`
      (return "NewEnumerator0"))
    (:`NewEnumerator1`
      (return "NewEnumerator1"))
    (:`NewEnumerator2`
      (return "NewEnumerator2"))
    (:`NewEnumerator3`
      (return "NewEnumerator3"))))

(fn `GetItemData`
  (returns (ItemData :type "/Game/Blueprints/Items/FItemData Structure"))
  (return (make `/Game/Blueprints/Items/FItemData` (`self.ItemName`) (`self.ItemType`) (`self.ItemQuantity`))))

(fn `GetItemType`
  (returns (ItemType :type "/Game/Blueprints/Items/EItemType Enum"))
  (return "NewEnumerator1"))

(fn `PlacePhoto`
  (params (PhotoREF :type "Actor Object Reference"))
  (bind _photopoint (`self.PhotoPoint`))
  (`self.K2_SetActorLocationAndRotation` PhotoREF (`SceneComponent.K2_GetComponentLocation` _photopoint) (`SceneComponent.K2_GetComponentRotation` _photopoint) false false)
  (bind _output_get (set `self.PhotoActor` PhotoREF))
  (message `/Game/Blueprints/Photos/BPI_Photo.ConnectVessel` _output_get self)
  (`self.DeactivateColliders`))

(fn `SetPhotoFailed`
  (bind _photoactor (`self.PhotoActor`))
  (`/Engine/EditorBlueprintResources/StandardMacros.IsValid` _photoactor
    (:`Is Valid`
      (message `/Game/Blueprints/Photos/BPI_Photo.ChangePhotoState` _photoactor "NewEnumerator4")
      (`ProgressBar.SetFillColorAndOpacity` (`/Game/UI/WBP_ProgressBar.ProgressBar` (`self.ProgressBarActor`)) (struct :`R` 0.854167 :`G` 0.025928 :`B` 0.059924 :`A` 1.0))
      (set `self.bIsOverexposing` false))))

(fn `UpdateProgressBar`
  (`ProgressBar.SetPercent` (`/Game/UI/WBP_ProgressBar.ProgressBar` (`self.ProgressBarActor`)) (`self.ProgressValue`)))

(fn `UserConstructionScript`
  (`parent.UserConstructionScript`))