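; BP_Door is an interactable door that swings open away from the player and closes on the next interaction.
; HandleInteraction alternates through a FlipFlop, setting IsOpen and playing or reversing a timeline that lerps the door's yaw in world rotation.
; On opening, a dot product of the actor's forward vector and direction to the player picks a ±90 degree swing.
; Item query functions return fixed placeholder values, with CanInteract and CanPickup both false.
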(event `/Game/Blueprints/Items/BPI_Interactable.HandleInteraction`
  (params (HeldItemREF :type "Actor Object Reference"))
  (`/Engine/EditorBlueprintResources/StandardMacros.FlipFlop`
    (:`A`
      (set `self.bIsOpen` true)
      (`self.SetDoorOpenAngle`)
      (bind (_direction _alpha) (`Timeline|OpenDoorTimeline` :!label _label)
        (:`Update`
          (`SceneComponent.K2_SetWorldRotation` (`self.Door`) (`KismetMathLibrary.MakeRotator` 0.0 0.0 (`KismetMathLibrary.Lerp` 0.0 (`self.DoorAngle`) _alpha)) false false))))
    (:`B`
      (set `self.bIsOpen` false)
      (goto _label :!via `Reverse`))))

(fn `CanInteract`
  (returns (CanInteract :type Boolean))
  (return false))

(fn `CanPickup`
  (returns (bCanPickup :type Boolean))
  (return false))

(fn `GetItemData`
  (returns (ItemData :type "/Game/Blueprints/Items/FItemData Structure"))
  (return (make `/Game/Blueprints/Items/FItemData` "")))

(fn `GetItemType`
  (returns (ItemType :type "/Game/Blueprints/Items/EItemType Enum"))
  (return "NewEnumerator4"))

(fn `SetDoorOpenAngle`
  ; Calculate DoorAngle based on dot product
  (set `self.DoorAngle` (`KismetMathLibrary.SelectFloat` -90.0 90.0 (>= (`KismetMathLibrary.Dot_VectorVector` (`KismetMathLibrary.GetDirectionUnitVector` (`self.K2_GetActorLocation`) (`self.K2_GetActorLocation` (`GameplayStatics.GetPlayerCharacter` 0))) (`self.GetActorForwardVector`)) 0.0))))

(fn `UserConstructionScript`)