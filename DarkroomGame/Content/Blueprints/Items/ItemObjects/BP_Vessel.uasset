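; Darkroom vessel item for one chemical (developer, stop bath, fixer or water) that advances photos through development phases.
; Once placed it cannot be picked up and can be filled by a matching liquid item, which it consumes.
; When filled, it accepts photos in the required state and phase, links them to itself, and advances their phase after an immersion timer.
; Exposure disables the vessel's collision until ClearValues restores it.
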(event `/Game/Blueprints/Items/BPI_Interactable.HandleInteraction`
  (params (HeldItemREF :type "Actor Object Reference"))
  (if (`KismetSystemLibrary.DoesImplementInterface` HeldItemREF "/Game/Blueprints/Items/BPI_Liquid.BPI_Liquid_C")
    (bind _bfilledsuccessful (`self.FillVessel` HeldItemREF))
    (if _bfilledsuccessful
      (`/Engine/EditorBlueprintResources/StandardMacros.IsValid` HeldItemREF
        (:`Is Valid`
          (`self.K2_DestroyActor` HeldItemREF))))
    (elif (`KismetSystemLibrary.DoesImplementInterface` HeldItemREF "/Game/Blueprints/Photos/BPI_Photo.BPI_Photo_C")
      (if (`self.bIsFilled`)
        (bind _photostate (message `/Game/Blueprints/Photos/BPI_Photo.GetPhotoState` HeldItemREF))
        (if (`|EnumEquality` _photostate "NewEnumerator1")
          (bind _photophase (message `/Game/Blueprints/Photos/BPI_Photo.GetPhotoPhase` HeldItemREF))
          (bind _photophase_2 (`self.GetAcceptedPhotoPhase`))
          (if (`|EnumEquality` _photophase _photophase_2)
            (`self.PlacePhoto` HeldItemREF)
            (`KismetSystemLibrary.K2_SetTimerDelegate` (delegate `CallExposePhoto`) (`self.ImmersionTimer`))))))))

(event `CallExposePhoto`
  (`self.DevelopPhoto` (`self.PhotoActor`)))

(event `/Game/Blueprints/Items/BPI_Interactable.ClearValues`
  (`self.ClearValuesFunction`))

(fn `CanInteract`
  (returns (CanInteract :type Boolean))
  (return true))

(fn `CanPickup`
  (returns (bCanPickup :type Boolean))
  (return (not (`self.bIsPlaced`))))

(fn `ClearValuesFunction`
  (`PrimitiveComponent.SetCollisionEnabled` (`self.HitBox`) "QueryAndPhysics")
  (`PrimitiveComponent.SetCollisionEnabled` (`self.LiquidMesh`) "QueryAndPhysics")
  (`PrimitiveComponent.SetCollisionEnabled` (`self.ItemMesh`) "QueryAndPhysics"))

(fn `DevelopPhoto`
  (params (PhotoToExpose :type "Actor Object Reference"))
  (switch `/Game/Blueprints/Items/EChemicalType` (`self.ChemicalType`)
    (:`NewEnumerator0`
      (message `/Game/Blueprints/Photos/BPI_Photo.ChangePhotoPhase` PhotoToExpose "NewEnumerator1"))
    (:`NewEnumerator1`
      (message `/Game/Blueprints/Photos/BPI_Photo.ChangePhotoPhase` PhotoToExpose "NewEnumerator2"))
    (:`NewEnumerator2`
      (message `/Game/Blueprints/Photos/BPI_Photo.ChangePhotoPhase` PhotoToExpose "NewEnumerator3"))
    (:`NewEnumerator3`
      (message `/Game/Blueprints/Photos/BPI_Photo.ChangePhotoPhase` PhotoToExpose "NewEnumerator4")))
  (`PrimitiveComponent.SetCollisionEnabled` (`self.HitBox`) "NoCollision")
  (`PrimitiveComponent.SetCollisionEnabled` (`self.LiquidMesh`) "NoCollision")
  (`PrimitiveComponent.SetCollisionEnabled` (`self.ItemMesh`) "NoCollision")
  (`KismetSystemLibrary.PrintString` "Photo changed phase!"))

(fn `FillVessel`
  (params (HeldItem :type "Object Object Reference"))
  (returns (bFilledSuccessful :type Boolean))
  (`/Engine/EditorBlueprintResources/StandardMacros.IsValid` HeldItem
    (:`Is Valid`
      (if (`self.bIsPlaced`)
        (if (`KismetSystemLibrary.DoesImplementInterface` HeldItem "/Game/Blueprints/Items/BPI_Liquid.BPI_Liquid_C")
          (bind _liquidtype (message `/Game/Blueprints/Items/BPI_Liquid.GetLiquidType` HeldItem))
          (if (`|EnumEquality` _liquidtype (`self.ChemicalType`))
            (`SceneComponent.SetVisibility` (`self.LiquidMesh`) true false)
            (set `self.bIsFilled` true)
            (return true)))))))

(fn `GetAcceptedPhotoPhase`
  (returns (PhotoPhase :type "/Game/Blueprints/Photos/EPhotoPhase Enum"))
  (switch `/Game/Blueprints/Items/EChemicalType` (`self.ChemicalType`)
    (:`NewEnumerator0`
      (return "NewEnumerator0"))
    (:`NewEnumerator1`
      (return "NewEnumerator1"))
    (:`NewEnumerator2`
      (return "NewEnumerator2"))
    (:`NewEnumerator3`
      (return "NewEnumerator3"))))

(fn `GetItemData`
  (returns (ItemData :type "/Game/Blueprints/Items/FItemData Structure"))
  (return (make `/Game/Blueprints/Items/FItemData` (`self.ItemName`) (`self.ItemType`) (`self.ItemQuantity`))))

(fn `GetItemType`
  (returns (ItemType :type "/Game/Blueprints/Items/EItemType Enum"))
  (return "NewEnumerator1"))

(fn `PlacePhoto`
  (params (PhotoREF :type "Actor Object Reference"))
  (bind _photopoint (`self.PhotoPoint`))
  (`self.K2_SetActorLocationAndRotation` PhotoREF (`SceneComponent.K2_GetComponentLocation` _photopoint) (`SceneComponent.K2_GetComponentRotation` _photopoint) false false)
  (bind _output_get (set `self.PhotoActor` PhotoREF))
  (message `/Game/Blueprints/Photos/BPI_Photo.ConnectVessel` _output_get self))

(fn `UserConstructionScript`
  (`parent.UserConstructionScript`))