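; Darkroom enlarger item that exposes a photo placed on it while its light is on.
; Interacting with a BPI_Photo item snaps it to PhotoPoint and links it back to the enlarger; otherwise interaction toggles the spotlight and indicator.
; With photo and light present, an exposure timer starts if GI_Main allows developing, and switching off cancels it.
; Exposure changes the photo's state and disables mesh collision until ClearValues resets the enlarger.
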(event `/Game/Blueprints/Items/BPI_Interactable.HandleInteraction`
  (params (HeldItemREF :type "Actor Object Reference"))
  (if (and (not (`KismetSystemLibrary.IsValid` (`self.PhotoActor`))) (`KismetSystemLibrary.DoesImplementInterface` HeldItemREF "/Game/Blueprints/Photos/BPI_Photo.BPI_Photo_C"))
    (`self.PlacePhoto` HeldItemREF)
    (if (`self.bIsOn`)
      (bind _asgi_main (cast `/Game/GI_Main` (`GameplayStatics.GetGameInstance`) :!label _label))
      (if (`/Game/GI_Main.bCanDevelopPhoto` _asgi_main)
        (bind _returnvalue (`KismetSystemLibrary.K2_SetTimerDelegate` (delegate `CallExposePhoto`) (`self.ExposureTimer`)))))
    (else
      (`self.ToggleEnlarger`)
      (`/Engine/EditorBlueprintResources/StandardMacros.IsValid` (`self.PhotoActor`)
        (:`Is Valid`
          (if (`self.bIsOn`)
            (goto _label)
            (else
              (`KismetSystemLibrary.K2_ClearAndInvalidateTimerHandle` _returnvalue))))))))

(event `CallExposePhoto`
  (`self.ExposePhoto` (`self.PhotoActor`)))

(event `/Game/Blueprints/Items/BPI_Interactable.ClearValues`
  (`self.ClearValuesFunction`))

(fn `ClearValuesFunction`
  (set `self.bHasPhoto` false)
  (set `self.bIsPhotoExposed` false)
  (set `self.PhotoActor` null)
  (`PrimitiveComponent.SetCollisionEnabled` (`self.ItemMesh`) "QueryAndPhysics"))

(fn `ExposePhoto`
  (params (PhotoToExpose :type "Actor Object Reference"))
  (message `/Game/Blueprints/Photos/BPI_Photo.ChangePhotoState` PhotoToExpose "NewEnumerator1")
  (set `self.bIsPhotoExposed` true)
  (`KismetSystemLibrary.PrintString` "Photo Exposed!")
  (`PrimitiveComponent.SetCollisionEnabled` (`self.ItemMesh`) "NoCollision"))

(fn `PlacePhoto`
  (params (PhotoREF :type "Actor Object Reference"))
  (bind _photopoint (`self.PhotoPoint`))
  (`self.K2_SetActorLocationAndRotation` PhotoREF (`SceneComponent.K2_GetComponentLocation` _photopoint) (`SceneComponent.K2_GetComponentRotation` _photopoint) false false)
  (bind _output_get (set `self.PhotoActor` PhotoREF))
  (message `/Game/Blueprints/Photos/BPI_Photo.ConnectEnlarger` _output_get self))

(fn `ToggleEnlarger`
  (if (not (`self.bIsOn`))
    (`SceneComponent.SetVisibility` (`self.SpotLight`) true false)
    (`PrimitiveComponent.SetMaterial` (`self.On/Off Light`) 0 "/Engine/EngineDebugMaterials/VertexColorViewMode_GreenOnly.VertexColorViewMode_GreenOnly")
    (set `self.bIsOn` true)
    (else
      (`SceneComponent.SetVisibility` (`self.SpotLight`) false false)
      (`PrimitiveComponent.SetMaterial` (`self.On/Off Light`) 0 "/Engine/VREditor/BasicMeshes/MI_Cube_03.MI_Cube_03")
      (set `self.bIsOn` false)))
  (`GameplayStatics.PlaySound2D` "/Engine/VREditor/Sounds/UI/Click_on_Button.Click_on_Button" 1.0 1.0 0.0 null null))

(fn `UserConstructionScript`
  (`parent.UserConstructionScript`))