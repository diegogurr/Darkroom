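; BP_CeilingLight is a ceiling spot light that starts dark and can be switched on and off.
; On BeginPlay it caches the SpotLight's authored intensity, then sets it to zero.
; The ToggleLight event flips IsOn, switches between the cached intensity and zero, and plays a non-spatialized flashlight switch sound.
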(event `self.ReceiveBeginPlay`
  (set `self.MaxLightIntensity` (`LightComponentBase.Intensity` (`self.SpotLight`)))
  (`LightComponent.SetIntensity` (`self.SpotLight`) 0.0))

(event `ToggleLight`
  (bind _output_get (set `self.IsOn` (not (`self.IsOn`))))
  (if _output_get
    (`LightComponent.SetIntensity` (`self.SpotLight`) (`self.MaxLightIntensity`))
    (else
      (`LightComponent.SetIntensity` (`self.SpotLight`) 0.0)))
  (`GameplayStatics.PlaySound2D` "/Engine/VREditor/Sounds/UI/Flashlight_Switch.Flashlight_Switch" 1.0 1.0 0.0 null null))

(fn `UserConstructionScript`)