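; BP_LampLight is a toggleable lamp that reports itself as a red light and identifies as a "Lamp" item.
; It caches the light's intensity at BeginPlay, starts dark, then switches between that intensity and zero when HandleInteraction calls ToggleLight.
; Each toggle plays a 2D switch sound and tells BP_LightManager to update lights.
; CanInteract and CanPickup both return false, while GetLightIsOn exposes the current state.
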(event `self.ReceiveBeginPlay`
  (set `self.MaxLightIntensity` (`LightComponentBase.Intensity` (`self.LampLight`)))
  (`LightComponent.SetIntensity` (`self.LampLight`) 0.0))

(event `/Game/Blueprints/Lights/BPI_Lights.ToggleLight`
  (bind _output_get (set `self.IsOn` (not (`self.IsOn`))))
  (if _output_get
    (`LightComponent.SetIntensity` (`self.LampLight`) (`self.MaxLightIntensity`))
    (else
      (`LightComponent.SetIntensity` (`self.LampLight`) 0.0)))
  (`GameplayStatics.PlaySound2D` "/Engine/VREditor/Sounds/UI/Flashlight_Switch.Flashlight_Switch" 1.0 1.0 0.0 null null)
  (bind _returnvalue (`GameplayStatics.GetActorOfClass` "/Game/Blueprints/Lights/BP_LightManager.BP_LightManager_C"))
  (`/Engine/EditorBlueprintResources/StandardMacros.IsValid` _returnvalue
    (:`Is Valid`
      (`/Game/Blueprints/Lights/BP_LightManager.UpdateLights` _returnvalue))))

(event `/Game/Blueprints/Items/BPI_Interactable.HandleInteraction`
  (params (HeldItemREF :type "Actor Object Reference"))
  (`self.ToggleLight`))

(fn `CanInteract`
  (returns (CanInteract :type Boolean))
  (return false))

(fn `CanPickup`
  (returns (bCanPickup :type Boolean))
  (return false))

(fn `GetItemData`
  (returns (ItemData :type "/Game/Blueprints/Items/FItemData Structure"))
  (return (make `/Game/Blueprints/Items/FItemData` "Lamp")))

(fn `GetItemType`
  (returns (ItemType :type "/Game/Blueprints/Items/EItemType Enum"))
  (return "NewEnumerator4"))

(fn `GetLightIsOn`
  (returns (bIsOn :type Boolean))
  (return (`self.IsOn`)))

(fn `IsARedLight`
  (returns (bIsRedLight :type Boolean))
  (return true))

(fn `UserConstructionScript`)