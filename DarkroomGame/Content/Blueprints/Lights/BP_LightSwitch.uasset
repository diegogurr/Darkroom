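; BP_LightSwitch is a light switch that toggles an array of linked lights when its interaction event fires.
; HandleInteraction messages each LightToToggle entry implementing BPI_Lights, then queries its new state to play an on or off 2D sound, once per light.
; Its item functions report a "Ceiling Light" item, and both CanInteract and CanPickup return false.
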(event `/Game/Blueprints/Items/BPI_Interactable.HandleInteraction`
  (params (HeldItemREF :type "Actor Object Reference"))
  (for _array_element (`self.LightToToggle`)
    (if (`KismetSystemLibrary.DoesImplementInterface` _array_element "/Game/Blueprints/Lights/BPI_Lights.BPI_Lights_C")
      (message `/Game/Blueprints/Lights/BPI_Lights.ToggleLight` _array_element)
      (bind _bison (message `/Game/Blueprints/Lights/BPI_Lights.GetLightIsOn` _array_element))
      (if _bison
        (`GameplayStatics.PlaySound2D` "/Game/Assets/Sounds/interruttore_luce_on.interruttore_luce_on" 1.0 1.0 0.0 null null)
        (else
          (`GameplayStatics.PlaySound2D` "/Game/Assets/Sounds/interruttore_luce_off.interruttore_luce_off" 1.0 1.0 0.0 null null))))))

(fn `CanInteract`
  (returns (CanInteract :type Boolean))
  (return false))

(fn `CanPickup`
  (returns (bCanPickup :type Boolean))
  (return false))

(fn `GetItemData`
  (returns (ItemData :type "/Game/Blueprints/Items/FItemData Structure"))
  (return (make `/Game/Blueprints/Items/FItemData` "Ceiling Light")))

(fn `GetItemType`
  (returns (ItemType :type "/Game/Blueprints/Items/EItemType Enum"))
  (return "NewEnumerator4"))

(fn `UserConstructionScript`)